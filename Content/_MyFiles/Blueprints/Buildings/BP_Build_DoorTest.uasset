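; BP_Build_DoorTest is a test door that swings open when BP_ThirdPersonCharacter enters its Box trigger.
; On entry, guarded by IsOpening, it disables StaticMesh1 collision and a timeline yaws the Arrow component toward -90 degrees.
; On exit, a second timeline repeatedly scales the Arrow's current rotation by its track rather than interpolating from a stored angle.
; The node that restores collision is unconnected, so collision stays off after first opening.
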(event `self.ReceiveBeginPlay`)

(event `self.Box.OnComponentBeginOverlap`
  (params (OverlappedComponent :type "PrimitiveComponent Object Reference") (OtherActor :type "Actor Object Reference") (OtherComp :type "PrimitiveComponent Object Reference") (OtherBodyIndex :type Integer) (bFromSweep :type Boolean) (SweepResult :type "HitResult Structure (by ref)"))
  (bind _asbp_third_person_character (cast `/Game/_MyFiles/Blueprints/BP_ThirdPersonCharacter` OtherActor))
  (`/Engine/EditorBlueprintResources/StandardMacros.IsValid` _asbp_third_person_character
    (:`Is Valid`
      (if (not (`self.bIsOpening`))
        (`PrimitiveComponent.SetCollisionEnabled` (`self.StaticMesh1`) "NoCollision")
        (set `self.bIsOpening` true)
        (bind (_direction _lerptrack) (`Timeline|LerpTimeline` :!via `PlayFromStart`)
          (:`Update`
            (`SceneComponent.K2_SetRelativeRotation` (`self.Arrow`) (* (`KismetMathLibrary.MakeRotator` 0.0 0.0 -90.0) _lerptrack) false false))
          (:`Finished`
            (set `self.bIsOpening` false)))))))

(event `self.Box.OnComponentEndOverlap`
  (params (OverlappedComponent :type "PrimitiveComponent Object Reference") (OtherActor :type "Actor Object Reference") (OtherComp :type "PrimitiveComponent Object Reference") (OtherBodyIndex :type Integer))
  (bind _arrow (`self.Arrow`))
  (bind _asbp_third_person_character (cast `/Game/_MyFiles/Blueprints/BP_ThirdPersonCharacter` OtherActor))
  (`/Engine/EditorBlueprintResources/StandardMacros.IsValid` _asbp_third_person_character
    (:`Is Valid`
      (set `self.bIsOpening` false)
      (bind (_direction _lerptrack) (`Timeline|Timeline` :!via `PlayFromStart`)
        (:`Update`
          (`SceneComponent.K2_SetRelativeRotation` _arrow (* (`SceneComponent.RelativeRotation` _arrow) _lerptrack) false false))))))

(fn `UserConstructionScript`)