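; BP_Build_Foundation is a foundation piece for a building system.
; It carries twelve box components in groups of four, named for foundation, wall and triangle foundation, which suggests snap points for those piece types.
; ReturnBoxes returns them all as one array.
; The event graph and construction script are empty, so the Blueprint has no other logic of its own.
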(fn `ReturnBoxes`
  (returns (Boxes :type "Array of BoxComponent Object Reference"))
  (return (`|MakeArray` (`self.Foundation`) (`self.Foundation1`) (`self.Foundation2`) (`self.Foundation3`) (`self.Wall`) (`self.Wall1`) (`self.Wall2`) (`self.Wall3`) (`self.TriFoundation`) (`self.TriFoundation1`) (`self.TriFoundation2`) (`self.TriFoundation3`))))

(fn `UserConstructionScript`)