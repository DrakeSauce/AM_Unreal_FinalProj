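; Player building component that toggles build mode (selection UI, cursor, character materials) and places buildings from a data table.
; A 0.1-second BuildCycle/BuildDelay loop camera-traces to position a ghost mesh, snapping to build boxes reported by the hit actor.
; A shrunken box trace tints the ghost green or red and sets CanBuild.
; SpawnBuild charges wood, stone and iron and spawns the actor, or toggles build mode when unaffordable.
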(event `self.ReceiveBeginPlay`
  (bind _asam_game_mode (cast `/Game/_MyFiles/Blueprints/AM_GameMode` (`GameplayStatics.GetGameMode`)))
  (set `self.As AM Game Mode` _asam_game_mode)
  (bind _asbp_third_person_character (cast `/Game/_MyFiles/Blueprints/BP_ThirdPersonCharacter` (`GameplayStatics.GetPlayerCharacter` 0)))
  (set `self.PlayerRef` _asbp_third_person_character)
  (bind _outrownames (`DataTableFunctionLibrary.GetDataTableRowNames` "/Game/_MyFiles/Blueprints/Buildings/BuildablesDB.BuildablesDB"))
  (for _array_element _outrownames
    (bind _returnvalue (`|GetDataTableRow` "/Game/_MyFiles/Blueprints/Buildings/BuildablesDB.BuildablesDB" _array_element)
      (:`then`
        (`KismetArrayLibrary.Array_Add` (`self.Buildables`) _returnvalue)))))

(event `BuildDelay`
  (bind _build_ghost (`self.Build Ghost`))
  (if (`self.bIsBuildModeOn`)
    (`KismetSystemLibrary.Delay` 0.1)
    (`self.BuildCycle`)
    (else
      (set `self.bIsBuildModeOn` false :!label _label)
      (set `self.bCanBuild` false)
      (`/Engine/EditorBlueprintResources/StandardMacros.IsValid` _build_ghost
        (:`Is Valid`
          (`/Game/_MyFiles/Blueprints/BP_ThirdPersonCharacter.DestroyComponent` (`self.PlayerRef`) _build_ghost))))))

(event `StopBuildMode`
  (goto _label))

(event `LaunchBuildMode`
  (bind _playerref (`self.PlayerRef`))
  (bind _playerref_2 (`self.PlayerRef`))
  (bind _mesh (`Character.Mesh` _playerref))
  (bind _mesh_2 (`Character.Mesh` _playerref_2))
  (if (`self.bIsBuildModeOn`)
    (set `Widget.Visibility` "Hidden" (`/Game/_MyFiles/Blueprints/AM_GameMode.FactorySelect` (`self.As AM Game Mode`)))
    (set `PlayerController.bShowMouseCursor` false (`GameplayStatics.GetPlayerController` 0))
    (`PrimitiveComponent.SetMaterial` _mesh 0 "/Game/_MyFiles/Player_Character/Model/Material/Ch44_Body.Ch44_Body")
    (`PrimitiveComponent.SetMaterial` _mesh 1 "/Game/_MyFiles/Player_Character/Model/Material/Ch44_body1.Ch44_body1")
    (`self.StopBuildMode`)
    (set `PrimitiveComponent.bGenerateOverlapEvents` true (`/Game/_MyFiles/Blueprints/BP_ThirdPersonCharacter.UITarget` _playerref))
    (else
      (set `self.bIsBuildModeOn` true)
      (set `Widget.Visibility` "Visible" (`/Game/_MyFiles/Blueprints/AM_GameMode.FactorySelect` (`self.As AM Game Mode`)))
      (set `PlayerController.bShowMouseCursor` true (`GameplayStatics.GetPlayerController` 0))
      (`PrimitiveComponent.SetMaterial` _mesh_2 0 "/Game/_MyFiles/Player_Character/Model/Material/Ch44_body2.Ch44_body2")
      (`PrimitiveComponent.SetMaterial` _mesh_2 1 "/Game/_MyFiles/Player_Character/Model/Material/Ch44_body2.Ch44_body2")
      (set `PrimitiveComponent.bGenerateOverlapEvents` false (`/Game/_MyFiles/Blueprints/BP_ThirdPersonCharacter.UITarget` _playerref_2)))))

(fn `BuildCycle`
  (bind _camera (`self.Camera`))
  (bind (_buildtransform_location _buildtransform_rotation _buildtransform_scale) (`KismetMathLibrary.BreakTransform` (`self.BuildTransform`)))
  (bind _build_ghost (`self.Build Ghost`))
  (bind _returnvalue (`SceneComponent.K2_GetComponentLocation` _camera))
  (bind _returnvalue_2 (`SceneComponent.GetForwardVector` _camera))
  (bind (_output_mesh _output_tracechannel) (break `/Game/_MyFiles/Blueprints/Buildings/S_Buildables` (`|GetArrayItem` (`self.Buildables`) (`self.BuildID`))))
  (bind (_outhit _returnvalue_3) (`KismetSystemLibrary.LineTraceSingle` (+ _returnvalue (* _returnvalue_2 350)) (+ _returnvalue (* _returnvalue_2 1000)) _output_tracechannel))
  (if _returnvalue_3
    (bind (_bblockinghit _binitialoverlap _time _distance _location _impactpoint _normal _impactnormal _physmat _hitactor _hitcomponent _hitbonename _bonename _hititem _elementindex _faceindex _tracestart _traceend) (`GameplayStatics.BreakHitResult` _outhit))
    (set `self.BuildTransform` (`KismetMathLibrary.MakeTransform` _impactpoint _buildtransform_rotation _buildtransform_scale))
    (set `self.Hit Actor` _hitactor)
    (set `self.Hit Component` _hitcomponent)
    (`/Engine/EditorBlueprintResources/StandardMacros.IsValid` _build_ghost
      (:`Is Valid`
        (bind (_found _transform) (`self.DetectBuildBoxes`))
        (if _found
          (set `self.BuildTransform` _transform))
        (bind _hit (`self.CheckForOverlap`))
        (if _hit
          (`self.GiveBuildColor` false)
          (else
            (`self.GiveBuildColor` true)))
        (`self.BuildDelay`))
      (:`Is Not Valid`
        (`self.SpawnBuildGhost` :!label _label)
        (`self.BuildDelay` :!label _label_2)))
    (else
      (set `self.BuildTransform` (`KismetMathLibrary.MakeTransform` _traceend _buildtransform_rotation _buildtransform_scale))
      (`/Engine/EditorBlueprintResources/StandardMacros.IsValid` _build_ghost
        (:`Is Valid`
          (`self.GiveBuildColor` false)
          (goto _label_2))
        (:`Is Not Valid`
          (goto _label))))))

(fn `ChangeMesh`
  (bind _output_mesh (break `/Game/_MyFiles/Blueprints/Buildings/S_Buildables` (`|GetArrayItem` (`self.Buildables`) (`self.BuildID`))))
  (`StaticMeshComponent.SetStaticMesh` (`self.Build Ghost`) _output_mesh))

(fn `CheckForOverlap`
  (returns (Hit :type Boolean))
  (bind (_origin _boxextent) (`KismetSystemLibrary.GetComponentBounds` (`self.Build Ghost`)))
  (bind (_outhit _returnvalue) (`KismetSystemLibrary.BoxTraceSingle` :`Start` _origin :`End` _origin :`HalfSize` (/ _boxextent 5.0) :`TraceChannel` "TraceTypeQuery1" :`DrawDebugType` "ForOneFrame"))
  (return _returnvalue))

(fn `DetectBuildBoxes`
  (returns (Found :type Boolean) (Transform :type "Transform Structure"))
  (locals (LocalFound :type Boolean))
  (bind _boxes (message `/Game/_MyFiles/Blueprints/Buildings/BuildableInterface.ReturnBoxes` (`self.Hit Actor`)))
  (for _array_element _boxes
    (if (== _array_element (`self.Hit Component`))
      (set `local.LocalFound` true)
      (break)))
  (return (`local.LocalFound`) (`SceneComponent.K2_GetComponentToWorld` (`self.Hit Component`))))

(fn `GiveBuildColor`
  (params (bIsGreen :type Boolean))
  (bind _build_ghost (`self.Build Ghost`))
  (set `self.bCanBuild` bIsGreen)
  (for _index (range (`PrimitiveComponent.GetNumMaterials` (`self.Build Ghost`)))
    (if bIsGreen
      (`PrimitiveComponent.SetMaterial` _build_ghost _index "/Game/_MyFiles/Material/GreenColor.GreenColor")
      (else
        (`PrimitiveComponent.SetMaterial` _build_ghost _index "/Game/_MyFiles/Material/RedColor.RedColor"))))
  (`SceneComponent.K2_SetWorldTransform` (`self.Build Ghost`) (`self.BuildTransform`) false false))

(fn `SpawnBuild`
  (bind _playerref (`self.PlayerRef`))
  (bind (_output_mesh _output_tracechannel _output_actor _output_name _output_woodcost _output_stonecost _output_ironcost) (break `/Game/_MyFiles/Blueprints/Buildings/S_Buildables` (`|GetArrayItem` (`self.Buildables`) (`self.BuildID`))))
  (bind _returnvalue (`ThirdPersonCharBase.CheckCanBuy` _playerref _output_woodcost _output_stonecost _output_ironcost))
  (if _returnvalue
    (`ThirdPersonCharBase.BuyItem` _playerref _output_woodcost _output_stonecost _output_ironcost)
    (`|SpawnActorFromClass` _output_actor (`self.BuildTransform`) "Undefined" "OverrideRootScale" null null)
    (else
      (`self.LaunchBuildMode`))))

(fn `SpawnBuildGhost`
  (bind _output_mesh (break `/Game/_MyFiles/Blueprints/Buildings/S_Buildables` (`|GetArrayItem` (`self.Buildables`) (`self.BuildID`))))
  (bind _returnvalue (`|AddComponentByClass` (`self.PlayerRef`) "/Script/Engine.StaticMeshComponent" false (`self.BuildTransform`)))
  (bind _output_get (set `self.Build Ghost` _returnvalue))
  (`StaticMeshComponent.SetStaticMesh` _output_get _output_mesh)
  (`PrimitiveComponent.SetCollisionEnabled` (`self.Build Ghost`) "NoCollision"))