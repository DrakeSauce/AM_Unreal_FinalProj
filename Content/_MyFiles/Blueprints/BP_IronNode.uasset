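; Iron resource node actor that displays its health, defense and resource name in a status widget and dissolves away when broken down.
; On initialization it fills the widget and hides it, then sphere overlaps show and hide it.
; PhysEvent runs once, disabling collision, swapping the mesh material and driving a dissolve timeline before destroying the actor.
; The dissolve writes to a shared Material Parameter Collection rather than a per-instance material.
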(event `self.InitializeEvent`
  (bind _aswbp_node_status (cast `/Game/_MyFiles/Blueprints/WBP_NodeStatus` (`WidgetComponent.GetWidget` (`self.NodeStatus_Widget`))))
  (bind _output_get (set `self.As WBP Node Status` _aswbp_node_status))
  (set `Widget.Visibility` "Hidden" _output_get)
  (`/Game/_MyFiles/Blueprints/WBP_NodeStatus.InitializeUI` _output_get (`self.health`) (`self.damageResist`) (`self.maxHealth`) "Iron"))

(event `self.Sphere.OnComponentBeginOverlap`
  (params (OverlappedComponent :type "PrimitiveComponent Object Reference") (OtherActor :type "Actor Object Reference") (OtherComp :type "PrimitiveComponent Object Reference") (OtherBodyIndex :type Integer) (bFromSweep :type Boolean) (SweepResult :type "HitResult Structure (by ref)"))
  (set `Widget.Visibility` "Visible" (`self.As WBP Node Status`)))

(event `self.Sphere.OnComponentEndOverlap`
  (params (OverlappedComponent :type "PrimitiveComponent Object Reference") (OtherActor :type "Actor Object Reference") (OtherComp :type "PrimitiveComponent Object Reference") (OtherBodyIndex :type Integer))
  (set `Widget.Visibility` "Hidden" (`self.As WBP Node Status`)))

(event `self.PhysEvent`
  (`/Engine/EditorBlueprintResources/StandardMacros.DoOnce` false
    (:`Completed`
      (`PrimitiveComponent.SetCollisionEnabled` (`self.StaticMesh`) "NoCollision")
      (`PrimitiveComponent.SetMaterial` (`self.StaticMesh`) 0 "/Game/_MyFiles/Material/Iron_Texture.Iron_Texture")
      (bind (_direction _lerpvalue) (`Timeline|LerpTimeline` :!via `PlayFromStart`)
        (:`Update`
          (`KismetMaterialLibrary.SetScalarParameterValue` "/Game/_MyFiles/Material/MPC_IronTexture.MPC_IronTexture" "Dissolve Amount" (`KismetMathLibrary.Lerp` 0.0 35.0 _lerpvalue)))
        (:`Finished`
          (`self.K2_DestroyActor`))))))

(fn `UserConstructionScript`)