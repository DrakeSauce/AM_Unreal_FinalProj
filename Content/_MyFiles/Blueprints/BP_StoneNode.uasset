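; BP_StoneNode is a stone resource node that crumbles and dissolves away when its destruction event fires.
; InitializeEvent fills its hidden WBP_NodeStatus widget with health, defense and the resource name.
; PhysEvent runs once, swapping the static mesh for a runtime-added Geometry Collection and applying a rock material after a short delay.
; A timeline then drives dissolve through the global MPC_RockTexture parameter collection before destroying the actor.
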(event `self.InitializeEvent`
  (bind _aswbp_node_status (cast `/Game/_MyFiles/Blueprints/WBP_NodeStatus` (`WidgetComponent.GetWidget` (`self.NodeStatus_Widget`))))
  (bind _output_get (set `self.As WBP Node Status` _aswbp_node_status))
  (set `Widget.Visibility` "Hidden" _output_get)
  (`/Game/_MyFiles/Blueprints/WBP_NodeStatus.InitializeUI` _output_get (`self.health`) (`self.damageResist`) (`self.maxHealth`) "Stone"))

(event `self.PhysEvent`
  (bind (_returnvalue_x _returnvalue_y _returnvalue_z) (`KismetMathLibrary.BreakVector` (`self.K2_GetActorLocation`)))
  (bind _staticmesh (`self.StaticMesh`))
  (`/Engine/EditorBlueprintResources/StandardMacros.DoOnce` false
    (:`Completed`
      (`SceneComponent.ToggleVisibility` _staticmesh false)
      (`PrimitiveComponent.SetCollisionEnabled` _staticmesh "NoCollision")
      (bind _returnvalue (`AddComponent|NODE_AddGeometryCollectionComponent-0` :`bManualAttachment` true :`RelativeTransform` (`KismetMathLibrary.Conv_VectorToTransform` (`KismetMathLibrary.MakeVector` _returnvalue_x _returnvalue_y (+ _returnvalue_z 10.0)))))
      (bind _output_get (set `self.Destruction` _returnvalue))
      (`KismetSystemLibrary.Delay` 1.0)
      (`PrimitiveComponent.SetMaterial` _output_get 0 "/Game/_MyFiles/Material/Rock_Texture_Inst.Rock_Texture_Inst")
      (`PrimitiveComponent.SetMaterial` _output_get 1 "/Game/_MyFiles/Material/Rock_Texture_Inst.Rock_Texture_Inst")
      (bind (_direction _lerpvalue) (`Timeline|LerpTimeline` :!via `PlayFromStart`)
        (:`Update`
          (`KismetMaterialLibrary.SetScalarParameterValue` "/Game/_MyFiles/Material/MPC_RockTexture.MPC_RockTexture" "Dissolve Amount" (`KismetMathLibrary.Lerp` 0.0 30.0 _lerpvalue)))
        (:`Finished`
          (`self.K2_DestroyActor`))))))

(fn `UserConstructionScript`)